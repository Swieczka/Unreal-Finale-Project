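; AudioManager is an actor that plays background music matching the current game state: Desert, City, Tavern or Combat.
; CheckCurrentState stores the state, picks that state's song group and passes it to PlaySong, skipping requests to change to the state already active.
; PlaySong fades in a random track on the AudioPlayer component.
; BeginPlay starts the music, and each finished track triggers another random pick for the current state.
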(event `self.ReceiveBeginPlay`
  (`self.Check Current State` (`self.Current State`)))

(event `self.AudioPlayer.OnAudioFinished`
  (`self.Check Current State` (`self.Current State`)))

(fn `Check Current State`
  (params (State :type "/Game/BluePrints/Enviro/GameState Enum" :default "NewEnumerator1") (Change :type Boolean))
  (locals (`Sound Group` :type "Array of SoundWave Object Reference"))
  (if (not (and (`|EnumEquality` (`self.Current State`) State) Change))
    (bind _output_get (set `self.Current State` State))
    (switch `/Game/BluePrints/Enviro/GameState` _output_get
      (:`NewEnumerator1`
        (set `local.Sound Group` (`self.Desert Music`)))
      (:`NewEnumerator2`
        (set `local.Sound Group` (`self.City Music`)))
      (:`NewEnumerator3`
        (set `local.Sound Group` (`self.Tavern Music`)))
      (:`NewEnumerator4`
        (set `local.Sound Group` (`self.Combat Music`))))
    (`self.Play Song` (`local.Sound Group`))))

(fn `Play Song`
  (params (`Sound Group` :type "Array of SoundWave Object Reference"))
  (bind _audioplayer (`self.AudioPlayer`))
  (`AudioComponent.SetSound` _audioplayer (`|GetArrayItem` `Sound Group` (`KismetMathLibrary.RandomIntegerInRange` 0 (- (`KismetArrayLibrary.Array_Length` `Sound Group`) 1))))
  (`AudioComponent.FadeIn` _audioplayer 0.25 1.0 0.0 "Linear"))

(fn `UserConstructionScript`)